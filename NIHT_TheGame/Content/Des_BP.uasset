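; Destructible cube actor that fractures under damage and explodes visually when its health runs out.
; AnyDamage forwards damage to the ShapeCubeDM destructible component with a fixed impulse, using the actor's location as both hit point and impulse direction.
; It then subtracts from CubeHealth and spawns a scaled-up P_Explosion emitter on every hit that leaves health at or below zero, without destroying the actor.
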(event EventBeginPlay)

(event Collision|EventActorBeginOverlap
  (params (OtherActor :type Actor%20Object%20Reference)))

(event EventTick
  (params (DeltaSeconds :type Float%20%28single-precision%29)))

(event Game|Damage|EventAnyDamage
  (params (Damage :type Float%20%28single-precision%29) (DamageType :type Damage%20Type%20Object%20Reference) (InstigatedBy :type Controller%20Object%20Reference) (DamageCauser :type Actor%20Object%20Reference))
  (bind _returnvalue (Transformation|GetActorLocation))
  (Class|DestructibleComponent|ApplyDamage (Variables|Default|GetShape_Cube_DM) Damage _returnvalue _returnvalue 1e+02)
  (bind _output_get (Variables|Default|SetcubeHealth (- (Variables|Default|GetcubeHealth) Damage)))
  (if (<= _output_get 0.0)
    (Effects|SpawnEmitteratLocation "/Game/StarterContent/Particles/P_Explosion.P_Explosion" (Transformation|GetActorLocation) (Transformation|GetActorRotation) "3.000000,3.000000,3.000000")))

(fn ConstructionScript)