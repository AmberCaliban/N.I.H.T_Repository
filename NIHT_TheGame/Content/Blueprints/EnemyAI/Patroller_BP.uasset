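; Patroller enemy that turns to face a third-person character it sees and fires energy bullets on a two-second cooldown.
; Any-damage and radial-damage events each reduce health and destroy it at zero, though only the former triggers the explosion.
; BeginPlay caches three marker positions and picks one at random, but the timeline that would lerp toward it and re-roll targets never runs.
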(event OnSeePawn(PawnSensing)
  (params (Pawn :type Pawn%20Object%20Reference))
  ;[1 0.5007 0.4916] Look and Shoot at Player
  (bind _asthird_person_character (Utilities|Casting|CastToThirdPersonCharacter Pawn))
  (Utilities|FlowControl|Sequence
    (:then_0
      (Transformation|SetActorRotation (Math|Rotator|FindLookatRotation (Transformation|GetActorLocation) (Transformation|GetActorLocation _asthird_person_character))))
    (:then_1
      (if (Variables|Default|GetspawnProjectile)
        (Game|SpawnActorfromClass "/Game/Blueprints/unpureEnergy_Bullet.unpureEnergy_Bullet_C" (Transformation|GetWorldTransform (Variables|Default|GetProjectileSpawnPoint)) "Undefined" 0 0)
        (Variables|Default|SetspawnProjectile false)
        (Utilities|FlowControl|Delay 2.0)
        (Variables|Default|SetspawnProjectile true)))))

(event EventBeginPlay
  ;[1 1 1] Setting Patrol points
  (Variables|Default|SetPatrol%20Points (Utilities|Array|MakeArray (Transformation|GetWorldLocation (Variables|Default|GetMovePosition1)) (Transformation|GetWorldLocation (Variables|Default|GetMovePosition2)) (Transformation|GetWorldLocation (Variables|Default|GetMovePosition3))))
  (CallFunction|GetRandomLocation))

(event Game|Damage|EventRadialDamage
  (params (DamageReceived :type Float%20%28single-precision%29) (DamageType :type Damage%20Type%20Object%20Reference) (Origin :type Vector :default "0, 0, 0") (HitInfo :type Hit%20Result%20Structure%20%28by%20ref%29) (InstigatedBy :type Controller%20Object%20Reference) (DamageCauser :type Actor%20Object%20Reference))
  ;[1 1 1] Explosive Damage Set-up
  (bind _output_get (Variables|Default|SetpatrollerHealth (- (Variables|Default|GetpatrollerHealth) DamageReceived)))
  (if (<= _output_get 0.0)
    (Utilities|FlowControl|Delay 0.5)
    (Actor|DestroyActor)))

(event Game|Damage|EventAnyDamage
  (params (Damage :type Float%20%28single-precision%29) (DamageType :type Damage%20Type%20Object%20Reference) (InstigatedBy :type Controller%20Object%20Reference) (DamageCauser :type Actor%20Object%20Reference))
  ;[1 1 1] Health & Damage system
  (bind _output_get (Variables|Default|SetpatrollerHealth (- (Variables|Default|GetpatrollerHealth) Damage)))
  (if (<= _output_get 0.0)
    (Components|Activation|Activate (Variables|Default|Getexplode) false)
    (Utilities|FlowControl|Delay 0.5)
    (Actor|DestroyActor)))

(fn ConstructionScript)

(fn GetRandomLocation
  (Variables|Default|SetCurrent%20Patrol%20Point (Math|Random|RandomInteger (Utilities|Array|Length (Variables|Default|GetPatrol%20Points)))))