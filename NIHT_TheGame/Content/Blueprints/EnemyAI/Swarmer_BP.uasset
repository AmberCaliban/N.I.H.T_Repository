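; Swarmer enemy that chases the player on sight and deals melee damage on contact.
; PawnSensing stores the seen ThirdPersonCharacter and starts AIMoveTo, whose immediate output runs an overlap-checked melee hit.
; The Enemy component's begin overlap also applies damage, while end overlap only resets an otherwise unused flag and prints debug text after a delay.
; Incoming damage drains ChargerHealth; at zero it activates Explode, then destroys the actor shortly after.
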(event OnSeePawn(PawnSensing)
  (params (Pawn :type Pawn%20Object%20Reference))
  ;[1 1 1] Chase after Player upon sensing
  (bind _asthird_person_character (Utilities|Casting|CastToThirdPersonCharacter Pawn))
  (bind _output_get (Variables|Default|Setplayer _asthird_person_character))
  (AI|AIMoveTo self "0, 0, 0" _output_get 5.0 false
    (:then
      (CallFunction|MeleeAttack))))

(event OnComponentBeginOverlap(Enemy)
  (params (OverlappedComponent :type Primitive%20Component%20Object%20Reference) (OtherActor :type Actor%20Object%20Reference) (OtherComp :type Primitive%20Component%20Object%20Reference) (OtherBodyIndex :type Integer) (bFromSweep :type Boolean) (SweepResult :type Hit%20Result%20Structure%20%28by%20ref%29))
  (bind _asthird_person_character (Utilities|Casting|CastToThirdPersonCharacter OtherActor))
  (Game|Damage|ApplyDamage _asthird_person_character (Variables|Default|GetmeleeDamage) 0 self))

(event OnComponentEndOverlap(Enemy)
  (params (OverlappedComponent :type Primitive%20Component%20Object%20Reference) (OtherActor :type Actor%20Object%20Reference) (OtherComp :type Primitive%20Component%20Object%20Reference) (OtherBodyIndex :type Integer))
  (Utilities|Casting|CastToThirdPersonCharacter OtherActor)
  (Utilities|FlowControl|Delay 1.0)
  (Variables|Default|SetmeleeComplete false)
  (Development|PrintString "stopped hitting player"))

(event Custom|Melee%20Attack
  (bind _player (Variables|Default|Getplayer))
  ;[1 1 1] Melee Damage Set-Up
  (if (Collision|IsOverlappingActor _player :!class /Script/Engine.Actor)
    (Game|Damage|ApplyDamage _player (Variables|Default|GetmeleeDamage) 0 0)))

(event Game|Damage|EventAnyDamage
  (params (Damage :type Float%20%28single-precision%29) (DamageType :type Damage%20Type%20Object%20Reference) (InstigatedBy :type Controller%20Object%20Reference) (DamageCauser :type Actor%20Object%20Reference))
  ;[1 1 1] Health & Damage system
  (bind _output_get (Variables|Default|SetchargerHealth (- (Variables|Default|GetchargerHealth) Damage)))
  (if (<= _output_get 0.0)
    (Components|Activation|Activate (Variables|Default|Getexplode) false)
    (Utilities|FlowControl|Delay 0.3)
    (Actor|DestroyActor)))

(fn ConstructionScript)