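; Enemy turret that spots the third-person player, turns to face them and shoots energy bullets until destroyed.
; Pawn sensing, after a short delay, drives a Rotation timeline that updates look-at rotation and spawns UnpureEnergy_Bullet from a spawn point, gated by a fire-rate cooldown.
; Any-damage and radial-damage events each reduce health and destroy the turret after a delay at zero, but only any-damage activates the explosion effect.
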(event OnSeePawn(PawnSensing)
  (params (Pawn :type Pawn%20Object%20Reference))
  ;[1 1 1] Looking at Player
  (Utilities|FlowControl|Delay 0.3)
  (if (not (Variables|/Game/ThirdPersonBP/Blueprints/ThirdPersonCharacter.ThirdPersonCharacter_C|GetisDead (Variables|Default|Getplayer)))
    (bind _asthird_person_character (Utilities|Casting|CastToThirdPersonCharacter Pawn))
    (Variables|Default|Setplayer _asthird_person_character)
    (Utilities|FlowControl|Sequence
      (:then_0
        (Timeline|Rotation Play
          (:Update
            (Transformation|SetActorRotation (Math|Rotator|FindLookatRotation (Transformation|GetActorLocation) (Transformation|GetActorLocation _asthird_person_character))))))
      (:then_1
        ;[1 1 1] Shooting Projectile
        (if (Variables|Default|GetspawnProjectile)
          (Game|SpawnActorfromClass "/Game/Blueprints/unpureEnergy_Bullet.unpureEnergy_Bullet_C" (Transformation|GetWorldTransform (Variables|Default|GetProjectileSpawnPoint)) "Undefined" 0 0)
          (Variables|Default|SetspawnProjectile false)
          (Utilities|FlowControl|Delay (Variables|Default|GetfireRate))
          (Variables|Default|SetspawnProjectile true))))))

(event EventBeginPlay
  (bind _asthird_person_character (Utilities|Casting|CastToThirdPersonCharacter (Game|GetPlayerCharacter 0)))
  (Variables|Default|Setplayer _asthird_person_character))

(event Game|Damage|EventAnyDamage
  (params (Damage :type Float%20%28single-precision%29) (DamageType :type Damage%20Type%20Object%20Reference) (InstigatedBy :type Controller%20Object%20Reference) (DamageCauser :type Actor%20Object%20Reference))
  ;[1 1 1] Health & Damage System
  (bind _output_get (Variables|Default|SetturretHealth (- (Variables|Default|GetturretHealth) Damage)))
  (if (<= _output_get 0.0) ; Check for 0 Health
    (Components|Activation|Activate (Variables|Default|Getexplode) false)
    (Utilities|FlowControl|Delay 0.5)
    (Actor|DestroyActor)))

(event Game|Damage|EventRadialDamage
  (params (DamageReceived :type Float%20%28single-precision%29) (DamageType :type Damage%20Type%20Object%20Reference) (Origin :type Vector :default "0, 0, 0") (HitInfo :type Hit%20Result%20Structure%20%28by%20ref%29) (InstigatedBy :type Controller%20Object%20Reference) (DamageCauser :type Actor%20Object%20Reference))
  ;[1 1 1] Explosive Damage Set-up
  (bind _output_get (Variables|Default|SetturretHealth (- (Variables|Default|GetturretHealth) DamageReceived)))
  (if (<= _output_get 0.0) ; Check for 0 Health
    (Utilities|FlowControl|Delay 0.5)
    (Actor|DestroyActor)))

(fn ConstructionScript)