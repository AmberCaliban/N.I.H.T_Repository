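; Two-phase boss enemy that turns toward the player on pawn sensing and picks attacks by random rolls.
; Phase one uses minigun bursts and rockets; a health band triggers phase two, which blows off the miniguns and uses rockets, bubble shield and charged shots.
; Bullet overlaps feed AnyDamage, with a double-damage weak point that the shield protects.
; Injury and death throw physics debris; radial damage kills without it.
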(event OnSeePawn(PawnSensing)
  (params (Pawn :type Pawn%20Object%20Reference))
  (bind _returnvalue (Math|Random|RandomIntegerinRange 0 100))
  (bind _returnvalue_2 (Math|Random|RandomIntegerinRange 0 100))
  (bind _player (Variables|Default|Getplayer))
  ;[1 1 1] Looking at Player
  (Utilities|FlowControl|Delay 0.3)
  (if (not (Variables|/Game/ThirdPersonBP/Blueprints/ThirdPersonCharacter.ThirdPersonCharacter_C|GetisDead _player))
    (bind _asthird_person_character (Utilities|Casting|CastToThirdPersonCharacter Pawn))
    (if (Utilities|IsValid _player)
      (Utilities|FlowControl|Sequence
        (:then_0
          (Timeline|Timeline_0 Play ; Help Smooth the Rotation
            (:Update
              (Transformation|SetActorRotation (Math|Rotator|FindLookatRotation (Transformation|GetActorLocation) (Transformation|GetActorLocation _asthird_person_character))))))
        (:then_1
          ;[1 1 1] Phase Handler - 1st Phase
          (if (Variables|Default|GetfirstPhase) ; 1st Phase
            (if (<= _returnvalue 40)
              (if (not (Variables|Default|GetminigunFiring))
                (CallFunction|MinigunBurst)
                (Utilities|FlowControl|Delay 5.0)
                (Variables|Default|SetspawnProjectile false)
                (Utilities|FlowControl|Delay 1.0)
                (Variables|Default|SetspawnProjectile true))
              (elif (and (> _returnvalue 90) (<= _returnvalue 100))
                (CallFunction|FireRockets)))
            (else
              ;[1 1 1] Phase Handler - 2nd Phase
              (if (Variables|Default|GetsecondPhase) ; 2nd Phase
                (Utilities|FlowControl|Sequence
                  (:then_0
                    (Utilities|FlowControl|DoOnce false
                      (:Completed
                        (CallFunction|2ndPhaseIndication))))
                  (:then_1
                    (if (<= _returnvalue_2 10)
                      (CallFunction|FireRockets)
                      (elif (Math|Boolean|ANDBoolean (not (Variables|Default|GetbubbleShieldActive)) (> _returnvalue_2 50) (<= _returnvalue_2 60))
                        (CallFunction|BubbleShield)
                        (elif (Math|Boolean|ANDBoolean (> _returnvalue_2 60) (<= _returnvalue_2 100) (not (Variables|Default|GetchargingShot)))
                          (CallFunction|ChargeShot)
                          (Development|PrintString "Charge Shot"))))))))))))))

(event OnComponentBeginOverlap(Enemy)
  (params (OverlappedComponent :type Primitive%20Component%20Object%20Reference) (OtherActor :type Actor%20Object%20Reference) (OtherComp :type Primitive%20Component%20Object%20Reference) (OtherBodyIndex :type Integer) (bFromSweep :type Boolean) (SweepResult :type Hit%20Result%20Structure%20%28by%20ref%29))
  (Utilities|Casting|CastTorifleBullet_BP OtherActor
    (:then
      (Development|PrintString "hit")
      (Game|Damage|ApplyDamage self (Variables|Default|GetassaultDamage) 0 0))
    (:CastFailed
      (Utilities|Casting|CastTosniperBullet_BP OtherActor)
      (Game|Damage|ApplyDamage self (Variables|Default|GetsniperDamage) 0 0))))

(event OnComponentBeginOverlap(WeakPointCollider)
  (params (OverlappedComponent :type Primitive%20Component%20Object%20Reference) (OtherActor :type Actor%20Object%20Reference) (OtherComp :type Primitive%20Component%20Object%20Reference) (OtherBodyIndex :type Integer) (bFromSweep :type Boolean) (SweepResult :type Hit%20Result%20Structure%20%28by%20ref%29))
  ;[1 1 1] Weak Point Set-Up
  (bind _asrifle_bullet_bp (Utilities|Casting|CastTorifleBullet_BP OtherActor)
    (:then
      (if (Variables|Default|GetbubbleShieldActive)
        _
        (else
          (Game|Damage|ApplyDamage self (* (Variables|Default|GetassaultDamage) 2.0) 0 _asrifle_bullet_bp)))
      (Effects|SpawnEmitteratLocation "/Game/StarterContent/Particles/P_Explosion.P_Explosion" (Transformation|GetActorLocation _asrifle_bullet_bp))
      (Actor|DestroyActor _asrifle_bullet_bp))
    (:CastFailed
      (bind _assniper_bullet_bp (Utilities|Casting|CastTosniperBullet_BP OtherActor))
      (if (Variables|Default|GetbubbleShieldActive)
        _
        (else
          (Game|Damage|ApplyDamage _assniper_bullet_bp (* (Variables|Default|GetsniperDamage) 2.0) 0 _assniper_bullet_bp)))
      (Actor|DestroyActor _assniper_bullet_bp))))

(event Custom|Fire%20Rockets
  (bind _rocket_spawn_point (Variables|Default|GetRocket%20Spawn%20Point))
  (bind _returnvalue (Transformation|GetWorldTransform _rocket_spawn_point))
  ;[1 1 1] Homing Missiles
  (Audio|PlaySoundatLocation "/Game/SFX/RocketLaunch_PH_SFX.RocketLaunch_PH_SFX" (Transformation|GetWorldLocation _rocket_spawn_point))
  (for _index (range 0 4)
    (Game|SpawnActorfromClass "/Game/Blueprints/rocket_BP.rocket_BP_C" (Math|Transform|MakeTransform (+ (.location _returnvalue) (Math|Vector|MakeVector (Math|Random|RandomFloatinRange -5e+01 5e+01) (Math|Random|RandomFloatinRange -5e+01 5e+01) 0.0)) (.rotation _returnvalue) (.scale _returnvalue)) "Undefined" 0 0)))

(event Custom|Laser%20Cutter
  (Collision|LineTraceForObjects (Transformation|GetWorldLocation (Variables|Default|GetWeakPoint)) (Math|Vector|GetForwardVector (Variables|Default|GetEnemy)) (Utilities|Array|MakeArray "ObjectTypeQuery1" "ObjectTypeQuery3") false 0 "ForDuration"))

(event Custom|Minigun%20Stop
  ;[1 1 1] Minigun Bursts
  (Utilities|FlowControl|Gate true) ; enters at Close
)

(event Custom|Minigun%20Burst
  ;[1 1 1] Minigun Bursts
  (Utilities|FlowControl|Sequence :!label _label
    (:then_0
      (goto _label_2 Open))
    (:then_1
      (Utilities|FlowControl|Gate true :!label _label_2
        (:Exit
          (if (Variables|Default|GetspawnProjectile)
            (Utilities|FlowControl|Sequence
              (:then_0
                (Utilities|FlowControl|RetriggerableDelay (Variables|Default|GetfireRate))
                (goto _label))
              (:then_1
                (Utilities|FlowControl|Sequence
                  (:then_0
                    (Game|SpawnActorfromClass "/Game/Blueprints/unpureEnergy_Bullet.unpureEnergy_Bullet_C" (Math|Transform|MakeTransform (+ (Transformation|GetWorldLocation (Variables|Default|GetMinigunSpawnPoint1)) (Math|Vector|MakeVector (Math|Random|RandomFloatinRange -8e+01 8e+01) (Math|Random|RandomFloatinRange 0.0 0.0) (Math|Random|RandomFloatinRange -6e+01 6e+01))) (Transformation|GetWorldRotation (Variables|Default|GetMinigunSpawnPoint1)) "1,1,1") "Undefined" 0 0))
                  (:then_1
                    (Game|SpawnActorfromClass "/Game/Blueprints/unpureEnergy_Bullet.unpureEnergy_Bullet_C" (Math|Transform|MakeTransform (+ (Transformation|GetWorldLocation (Variables|Default|GetMinigunSpawnPoint2)) (Math|Vector|MakeVector (Math|Random|RandomFloatinRange -8e+01 8e+01) (Math|Random|RandomFloatinRange 0.0 0.0) (Math|Random|RandomFloatinRange -6e+01 6e+01))) (Transformation|GetWorldRotation (Variables|Default|GetMinigunSpawnPoint2)) "1,1,1") "Undefined" 0 0)))))))))))

(event Custom|Bubble%20Shield
  (bind _weakpoint (Variables|Default|GetWeakPoint))
  (bind _relativelocation (Variables|/Script/Engine.SceneComponent|GetRelativeLocation _weakpoint))
  (bind (_x _y _z) (Math|Vector|BreakVector _relativelocation))
  (Effects|SpawnEmitterAttached "/Game/VFX/BubbleShield_VFX.BubbleShield_VFX" _weakpoint "None" (Math|Vector|MakeVector (+ _x -3e+02) _y (+ _z 2e+02)) "0, 0, 0" "0.500000,0.500000,0.500000")
  (Variables|Default|SetbubbleShieldActive true)
  (Utilities|FlowControl|Delay 7.0)
  (Development|PrintString "bubble shield is off")
  (Variables|Default|SetbubbleShieldActive false))

(event Custom|Fire%20Charged%20Shot
  (bind _chargedparticle (Variables|Default|GetchargedParticle))
  (bind _projectilemovement (Variables|/Game/Blueprints/chargedUnpureEnergyBullet_BP.chargedUnpureEnergyBullet_BP_C|GetProjectileMovement _chargedparticle))
  (Transformation|DetachFromActor _chargedparticle "KeepWorld" "KeepWorld" "KeepWorld")
  (Variables|/Script/Engine.MovementComponent|SetVelocity _projectilemovement (* (Math|Vector|GetForwardVector (Variables|Default|GetEnemy)) 2e+03))
  (Components|Activation|Activate _projectilemovement false))

(event Custom|Stop%20Charging
  (Variables|Default|SetchargeTime 0.0)
  (Variables|Default|SetchargingShot false)
  (Timeline|ChargeBlaster Stop
    (:Charge
      (Variables|Default|SetchargingShot true)
      (if (< (Variables|Default|GetchargeTime) 1e+01)
        (bind _output_get (Variables|Default|SetchargeTime (+ (Variables|Default|GetchargeTime) 0.5)))
        (Development|PrintString (Utilities|String|ToString(Float) _output_get))
        (Transformation|SetActorScale3D (Variables|Default|GetchargedParticle) (Math|Vector|Lerp(Vector) (Transformation|GetActorScale3D (Variables|Default|GetchargedParticle)) (Math|Conversions|ToVector(Float) (Variables|Default|GetchargeTime)) 0.0))
        (CallFunction|FireChargedShot)
        (else
          (CallFunction|FireChargedShot))))))

(event Custom|2nd%20Phase%20Indication
  (bind _minigun1 (Variables|Default|GetMiniGun1))
  (bind _minigun2 (Variables|Default|GetMinigun2))
  ;[1 1 1] Indicators for 2nd Phase
  (Utilities|FlowControl|Sequence
    (:then_0
      (Effects|SpawnEmitteratLocation "/Game/StarterContent/Particles/P_Explosion.P_Explosion" (Transformation|GetWorldLocation (Variables|Default|GetMiniGun1)) "0, 0, 0" "2.000000,2.000000,2.000000")
      (Physics|SetSimulatePhysics (Variables|Default|GetMiniGun1) true)
      (Effects|SpawnEmitterAttached "/Game/StarterContent/Particles/P_Fire.P_Fire" _minigun1 "None" (Variables|/Script/Engine.SceneComponent|GetRelativeLocation _minigun1) "0, 0, 0" "4.000000,4.000000,4.000000"))
    (:then_1
      (Effects|SpawnEmitteratLocation "/Game/StarterContent/Particles/P_Explosion.P_Explosion" (Transformation|GetWorldLocation (Variables|Default|GetMinigun2)) "0, 0, 0" "2.000000,2.000000,2.000000")
      (Physics|SetSimulatePhysics (Variables|Default|GetMinigun2) true)
      (Effects|SpawnEmitterAttached "/Game/StarterContent/Particles/P_Fire.P_Fire" _minigun2 "None" (Variables|/Script/Engine.SceneComponent|GetRelativeLocation _minigun2) "0, 0, 0" "4.000000,4.000000,4.000000"))))

(event Custom|Charge%20Shot
  (bind _chargespot (Variables|Default|GetChargeSpot))
  (bind _returnvalue (Game|SpawnActorfromClass "/Game/Blueprints/chargedUnpureEnergyBullet_BP.chargedUnpureEnergyBullet_BP_C" (Math|Transform|MakeTransform (Transformation|GetWorldLocation _chargespot) (Transformation|GetWorldRotation _chargespot) "1,1,1") "Undefined" 0 0))
  (bind _output_get (Variables|Default|SetchargedParticle _returnvalue))
  (Transformation|AttachComponentToComponent _output_get (Variables|Default|GetChargeSpot) "None" "KeepWorld" "KeepWorld" "KeepWorld" true)
  (Timeline|ChargeBlaster PlayFromStart
    (:Charge
      (Variables|Default|SetchargingShot true)
      (if (< (Variables|Default|GetchargeTime) 1e+01)
        (bind _output_get_2 (Variables|Default|SetchargeTime (+ (Variables|Default|GetchargeTime) 0.5)))
        (Development|PrintString (Utilities|String|ToString(Float) _output_get_2))
        (Transformation|SetActorScale3D (Variables|Default|GetchargedParticle) (Math|Vector|Lerp(Vector) (Transformation|GetActorScale3D (Variables|Default|GetchargedParticle)) (Math|Conversions|ToVector(Float) (Variables|Default|GetchargeTime)) 0.0))
        (CallFunction|FireChargedShot)
        (else
          (CallFunction|FireChargedShot))))))

(event EventBeginPlay
  (bind _asthird_person_character (Utilities|Casting|CastToThirdPersonCharacter (Game|GetPlayerCharacter 0)))
  (Variables|Default|Setplayer _asthird_person_character))

(event Game|Damage|EventAnyDamage
  (params (Damage :type Float%20%28single-precision%29) (DamageType :type Damage%20Type%20Object%20Reference) (InstigatedBy :type Controller%20Object%20Reference) (DamageCauser :type Actor%20Object%20Reference))
  (bind _returnvalue (Transformation|GetActorLocation))
  ;[1 1 1] Health & Damage System
  (bind _output_get (Variables|Default|SetbossHealth (- (Variables|Default|GetbossHealth) Damage)))
  (if (<= _output_get 0.0) ; Check for 0 Health
    (Utilities|FlowControl|Delay 0.5)
    (Effects|SpawnEmitteratLocation "/Game/StarterContent/Particles/P_Explosion.P_Explosion" _returnvalue "0, 0, 0" "5.000000,5.000000,5.000000")
    (Audio|PlaySoundatLocation "/Game/StarterContent/Audio/Explosion02.Explosion02" _returnvalue)
    (CallFunction|Death)
    (elif (and (>= (Variables|Default|GetbossHealth) 1.4e+03) (<= (Variables|Default|GetbossHealth) 1.5e+03)) ; Check if 2nd Phase
      (Development|PrintString (Utilities|String|Append "Boss HP:" (Utilities|String|ToString(Float) (Variables|Default|GetbossHealth))))
      (CallFunction|Injured)
      (Utilities|FlowControl|DoOnce false
        (:Completed
          (Variables|Default|SetsecondPhase true)
          (Variables|Default|SetfirstPhase false)
          (Development|PrintString "Entering 2nd Phase")
          (Components|Activation|Activate (Variables|Default|GetFire) false))))))

(event Game|Damage|EventRadialDamage
  (params (DamageReceived :type Float%20%28single-precision%29) (DamageType :type Damage%20Type%20Object%20Reference) (Origin :type Vector :default "0, 0, 0") (HitInfo :type Hit%20Result%20Structure%20%28by%20ref%29) (InstigatedBy :type Controller%20Object%20Reference) (DamageCauser :type Actor%20Object%20Reference))
  ;[1 1 1] Explosive Damage Set-up
  (bind _output_get (Variables|Default|SetbossHealth (- (Variables|Default|GetbossHealth) DamageReceived)))
  (if (<= _output_get 0.0) ; Check for 0 Health
    (Utilities|FlowControl|Delay 0.5)
    (Actor|DestroyActor)))

(fn ConstructionScript)

(fn Death
  (bind _returnvalue (Math|Random|RandomFloatinRange 5.0 1e+01))
  (for _index (range 0 15)
    (bind _returnvalue_2 (Game|SpawnActorfromClass "/Game/Blueprints/bossDebris_BP.bossDebris_BP_C" (Math|Transform|MakeTransform (Transformation|GetActorLocation) (Transformation|GetActorRotation) (Math|Vector|MakeVector _returnvalue _returnvalue _returnvalue)) "Undefined" 0 0))
    (Physics|AddImpulse (Variables|/Game/Blueprints/bossDebris_BP.bossDebris_BP_C|GetStaticMesh _returnvalue_2) (Math|Vector|MakeVector (Math|Random|RandomFloatinRange -2e+03 2e+03) (Math|Random|RandomFloatinRange -2e+03 2e+03) (Math|Random|RandomFloatinRange 0.0 3e+03)) "None" false)
    (Actor|DestroyActor)))

(fn Injured
  (bind _returnvalue (Math|Random|RandomFloatinRange 1.0 3.0))
  (for _index (range 0 9)
    (bind _returnvalue_2 (Game|SpawnActorfromClass "/Game/Blueprints/bossDebris_BP.bossDebris_BP_C" (Math|Transform|MakeTransform (Transformation|GetActorLocation) (Transformation|GetActorRotation) (Math|Vector|MakeVector _returnvalue _returnvalue _returnvalue)) "Undefined" 0 0))
    (Physics|AddImpulse (Variables|/Game/Blueprints/bossDebris_BP.bossDebris_BP_C|GetStaticMesh _returnvalue_2) (Math|Vector|MakeVector (Math|Random|RandomFloatinRange -1e+03 1e+03) (Math|Random|RandomFloatinRange -1e+03 1e+03) (Math|Random|RandomFloatinRange 0.0 2e+03)) "None" false)))