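; Shotgun weapon actor for the player's ThirdPersonCharacter, handling firing, ammo, reloading and the pickup prompt.
; Trigger events drive a gated fire path that spends a shell and line-traces five randomly spread pellets from the camera, tighter or wider by aim state.
; Hits spawn RifleBullet_BP from the muzzle toward the impact, with a delayed flag limiting fire rate.
; Sphere overlap toggles pickup prompt and input; Reload refills the clip from reserve shells.
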(event OnComponentBeginOverlap(Sphere1)
  (params (OverlappedComponent :type Primitive%20Component%20Object%20Reference) (OtherActor :type Actor%20Object%20Reference) (OtherComp :type Primitive%20Component%20Object%20Reference) (OtherBodyIndex :type Integer) (bFromSweep :type Boolean) (SweepResult :type Hit%20Result%20Structure%20%28by%20ref%29))
  ;[1 1 1] Pick-up set-up & Prompt
  (Input|EnableInput (Game|GetPlayerController 0))
  (if (not (Variables|/Game/ThirdPersonBP/Blueprints/ThirdPersonCharacter.ThirdPersonCharacter_C|GetshotgunEquipped (Variables|Default|Getplayer)))
    (Rendering|SetVisibility (Variables|Default|GetPick%20up) true false)
    (Variables|/Game/ThirdPersonBP/Blueprints/ThirdPersonCharacter.ThirdPersonCharacter_C|SetcanPickUpSG (Variables|Default|Getplayer) true)))

(event OnComponentEndOverlap(Sphere1)
  (params (OverlappedComponent :type Primitive%20Component%20Object%20Reference) (OtherActor :type Actor%20Object%20Reference) (OtherComp :type Primitive%20Component%20Object%20Reference) (OtherBodyIndex :type Integer))
  ;[1 1 1] Pick-up set-up & Prompt
  (Input|DisableInput (Game|GetPlayerController 0))
  (Rendering|SetVisibility (Variables|Default|GetPick%20up) false false)
  (Variables|/Game/ThirdPersonBP/Blueprints/ThirdPersonCharacter.ThirdPersonCharacter_C|SetcanPickUpSG (Variables|Default|Getplayer) false))

(event Custom|pullTrigger
  (bind _player (Variables|Default|Getplayer))
  (bind _skeletalmesh (Variables|Default|GetSkeletalMesh))
  (bind _returnvalue (Transformation|GetSocketLocation _skeletalmesh "Muzzle"))
  (bind _followcamera (Variables|/Game/ThirdPersonBP/Blueprints/ThirdPersonCharacter.ThirdPersonCharacter_C|GetFollowCamera _player))
  (bind _returnvalue_2 (Transformation|GetWorldLocation _followcamera))
  (bind _returnvalue_3 (Math|Vector|GetForwardVector _followcamera))
  (bind _returnvalue_4 (* _returnvalue_3 1e+04))
  (bind _returnvalue_5 (+ _returnvalue_4 _returnvalue_2))
  (bind (_x _y _z) (Math|Vector|BreakVector _returnvalue_5))
  ;[1 1 1] Firing Projectile
  (Utilities|FlowControl|Sequence
    (:then_0
      (goto _label Open))
    (:then_1
      (Utilities|FlowControl|Gate true :!label _label
        (:Exit
          (Utilities|FlowControl|Sequence
            (:then_0
              (Utilities|FlowControl|RetriggerableDelay 4.0) ; Allow gun to be spammable
              (goto _label))
            (:then_1
              (if (Variables|Default|GetspawnProjectile)
                (if (Math|Boolean|Equal(Boolean) (Variables|/Game/ThirdPersonBP/Blueprints/ThirdPersonCharacter.ThirdPersonCharacter_C|GetisReloading (Variables|Default|Getplayer)) false)
                  (if (<= (Variables|Default|GetshellInClip) 0)
                    (Audio|PlaySoundatLocation "/Game/SFX/ARFireDry_PH_SFX.ARFireDry_PH_SFX" (Transformation|GetActorLocation))
                    (else
                      (Variables|Default|SetshellInClip (- (Variables|Default|GetshellInClip) 1))
                      (if (Variables|/Game/ThirdPersonBP/Blueprints/ThirdPersonCharacter.ThirdPersonCharacter_C|GetisAiming (Variables|Default|Getplayer)) ; Check if Player is ADS
                        (Variables|Default|SetshotSpreadMax (Variables|Default|GetaimShotSpreadMax))
                        (Variables|Default|SetshotSpreadMin (Variables|Default|GetaimShotSpreadMin))
                        (else
                          (Variables|Default|SetshotSpreadMax (Variables|Default|GethipShotSpreadMax))
                          (Variables|Default|SetshotSpreadMin (Variables|Default|GethipShotSpreadMin))))
                      (Audio|PlaySoundatLocation "/Game/SFX/SGFire_PH_SFX.SGFire_PH_SFX" (Transformation|GetSocketLocation (Variables|Default|GetSkeletalMesh) "Muzzle"))
                      (for _index (range 0 4)
                        (bind (_outhit _returnvalue_6) (Collision|LineTraceByChannel _returnvalue_2 (Math|Vector|MakeVector (+ _x (Math|Random|RandomFloatinRange (Variables|Default|GetshotSpreadMin) (Variables|Default|GetshotSpreadMax))) (+ _y (Math|Random|RandomFloatinRange (Variables|Default|GetshotSpreadMin) (Variables|Default|GetshotSpreadMax))) (+ _z (Math|Random|RandomFloatinRange (Variables|Default|GetshotSpreadMin) (Variables|Default|GetshotSpreadMax)))) "TraceTypeQuery1" false 0 "ForDuration")) ; Calculate bullet trajectory
                        (if _returnvalue_6
                          (Game|SpawnActorfromClass "/Game/Blueprints/Bullets/rifleBullet_BP.rifleBullet_BP_C" (Math|Transform|MakeTransform _returnvalue (Math|Rotator|FindLookatRotation _returnvalue (Math|Vector|SelectVector (.ImpactPoint (Collision|BreakHitResult _outhit)) (.TraceEnd (Collision|BreakHitResult _outhit)) _returnvalue_6))) "Undefined" 0 0)
                          (Variables|Default|SetspawnProjectile false)
                          (Utilities|FlowControl|Delay 1.5) ; Prevent Spamming
                          (Variables|Default|SetspawnProjectile true)))))
                  (else
                    (Development|PrintString "Cannot shoot while reloading" true false "(R=1.000000,G=0.046797,B=0.118639,A=1.000000)")))))))))))

(event Custom|releaseTrigger
  (bind _player (Variables|Default|Getplayer))
  (bind _skeletalmesh (Variables|Default|GetSkeletalMesh))
  (bind _returnvalue (Transformation|GetSocketLocation _skeletalmesh "Muzzle"))
  (bind _followcamera (Variables|/Game/ThirdPersonBP/Blueprints/ThirdPersonCharacter.ThirdPersonCharacter_C|GetFollowCamera _player))
  (bind _returnvalue_2 (Transformation|GetWorldLocation _followcamera))
  (bind _returnvalue_3 (Math|Vector|GetForwardVector _followcamera))
  (bind _returnvalue_4 (* _returnvalue_3 1e+04))
  (bind _returnvalue_5 (+ _returnvalue_4 _returnvalue_2))
  (bind (_x _y _z) (Math|Vector|BreakVector _returnvalue_5))
  ;[1 1 1] Firing Projectile
  (Utilities|FlowControl|Gate true) ; enters at Close
)

(event EventBeginPlay
  (bind _asthird_person_character (Utilities|Casting|CastToThirdPersonCharacter (Game|GetPlayerCharacter 0)))
  (Variables|Default|Setplayer _asthird_person_character))

(fn ConstructionScript)

(fn Reload
  (if (> (Variables|Default|GetmaxShotgunShell) 0)
    (if (not (== (Variables|Default|GetshellInClip) (Variables|Default|GetclipSize)))
      (if (> (Variables|Default|GetmaxShotgunShell) (Variables|Default|GetclipSize))
        (bind _asthird_person_character (Utilities|Casting|CastToThirdPersonCharacter (Game|GetPlayerCharacter 0)))
        (bind _output_get (Variables|/Game/ThirdPersonBP/Blueprints/ThirdPersonCharacter.ThirdPersonCharacter_C|SetisReloading _asthird_person_character true))
        (if (and (< (Variables|Default|GetshellInClip) (Variables|Default|GetclipSize)) (> (Variables|Default|GetshellInClip) 0))
          (Variables|Default|SetmaxShotgunShell (- (Variables|Default|GetmaxShotgunShell) 1))
          (Variables|Default|SetshellInClip (Variables|Default|GetclipSize))
          (return _output_get false)
          (elif (<= (Variables|Default|GetshellInClip) 0)
            (Variables|Default|SetmaxShotgunShell (- (Variables|Default|GetmaxShotgunShell) (Variables|Default|GetclipSize)))
            (Variables|Default|SetshellInClip (Variables|Default|GetclipSize))
            (return _output_get false)))
        (else
          (Variables|Default|SetshellInClip (Variables|Default|GetmaxShotgunShell))
          (Variables|Default|SetmaxShotgunShell 0)
          (bind _asthird_person_character_2 (Utilities|Casting|CastToThirdPersonCharacter (Game|GetPlayerCharacter 0)))
          (bind _output_get_2 (Variables|/Game/ThirdPersonBP/Blueprints/ThirdPersonCharacter.ThirdPersonCharacter_C|SetisReloading _asthird_person_character_2 true))
          (return false _output_get_2))))))