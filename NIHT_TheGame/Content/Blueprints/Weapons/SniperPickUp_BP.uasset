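; Sniper rifle pickup actor that shows a pickup prompt when the player character is in range.
; BeginPlay caches the player's ThirdPersonCharacter.
; Sphere overlaps toggle input on the actor, the PickUp prompt's visibility and the cached character's CanPickUpSR flag.
; An Equipped check suppresses the prompt and flag on entry; the pickup action itself is not handled in these graphs.
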(event OnComponentBeginOverlap(Sphere1)
  (params (OverlappedComponent :type Primitive%20Component%20Object%20Reference) (OtherActor :type Actor%20Object%20Reference) (OtherComp :type Primitive%20Component%20Object%20Reference) (OtherBodyIndex :type Integer) (bFromSweep :type Boolean) (SweepResult :type Hit%20Result%20Structure%20%28by%20ref%29))
  ;[1 1 1] Pick-up set-up & Prompt
  (Utilities|Casting|CastToThirdPersonCharacter OtherActor)
  (Input|EnableInput (Game|GetPlayerController 0))
  (if (not (Variables|Default|Getequipped))
    (Rendering|SetVisibility (Variables|Default|GetPick%20up) true false)
    (Variables|/Game/ThirdPersonBP/Blueprints/ThirdPersonCharacter.ThirdPersonCharacter_C|SetcanPickUpSR (Variables|Default|Getcharacter) true)))

(event OnComponentEndOverlap(Sphere1)
  (params (OverlappedComponent :type Primitive%20Component%20Object%20Reference) (OtherActor :type Actor%20Object%20Reference) (OtherComp :type Primitive%20Component%20Object%20Reference) (OtherBodyIndex :type Integer))
  ;[1 1 1] Pick-up set-up & Prompt
  (Utilities|Casting|CastToThirdPersonCharacter OtherActor)
  (Input|DisableInput (Game|GetPlayerController 0))
  (Rendering|SetVisibility (Variables|Default|GetPick%20up) false false)
  (Variables|/Game/ThirdPersonBP/Blueprints/ThirdPersonCharacter.ThirdPersonCharacter_C|SetcanPickUpSR (Variables|Default|Getcharacter) false))

(event EventBeginPlay
  (bind _asthird_person_character (Utilities|Casting|CastToThirdPersonCharacter (Game|GetPlayerCharacter 0)))
  (Variables|Default|Setcharacter _asthird_person_character))

(fn ConstructionScript)