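; Sniper rifle weapon Blueprint that fires SniperBullet_BP projectiles for the player's ThirdPersonCharacter and manages its ammo.
; Trigger pulls line-trace from the follow camera with aim or hip random spread, spawning a bullet aimed from the muzzle at the impact only on a hit.
; A flag and Delay enforce cocking time between shots, while reloading or an empty clip blocks firing.
; Reload refills the clip from reserve ammo and sets the player's IsReloading.
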(event Custom|pullTrigger
  (bind _projectilespawnpoint (Variables|Default|GetProjectileSpawnPoint))
  (bind _player (Variables|Default|Getplayer))
  (bind _returnvalue (Transformation|GetWorldLocation _projectilespawnpoint))
  (bind _followcamera (Variables|/Game/ThirdPersonBP/Blueprints/ThirdPersonCharacter.ThirdPersonCharacter_C|GetFollowCamera _player))
  (bind _returnvalue_2 (Math|Vector|GetForwardVector _followcamera))
  (bind _returnvalue_3 (Transformation|GetWorldLocation _followcamera))
  (bind _returnvalue_4 (* _returnvalue_2 1e+04))
  (bind _returnvalue_5 (+ _returnvalue_3 _returnvalue_4))
  (bind (_x _y _z) (Math|Vector|BreakVector _returnvalue_5))
  ;[1 1 1] Firing Projectile
  (Utilities|FlowControl|Sequence
    (:then_0
      (goto _label Open))
    (:then_1
      (Utilities|FlowControl|Gate true :!label _label
        (:Exit
          (Utilities|FlowControl|Sequence
            (:then_0
              (if (Variables|Default|GetspawnProjectile)
                (if (Math|Boolean|Equal(Boolean) (Variables|/Game/ThirdPersonBP/Blueprints/ThirdPersonCharacter.ThirdPersonCharacter_C|GetisReloading (Variables|Default|Getplayer)) false)
                  (if (<= (Variables|Default|GetlongBulletInClip) 0)
                    (Development|PrintString "Sniper is Empty" true false "(R=1.000000,G=0.059502,B=0.090399,A=1.000000)")
                    (Audio|PlaySoundatLocation "/Game/SFX/ARFireDry_PH_SFX.ARFireDry_PH_SFX" (Transformation|GetActorLocation))
                    (else
                      (if (Variables|/Game/ThirdPersonBP/Blueprints/ThirdPersonCharacter.ThirdPersonCharacter_C|GetisAiming (Variables|Default|Getplayer))
                        (Variables|Default|SetshotSpreadMax (Variables|Default|GetaimShotSpreadMax))
                        (Variables|Default|SetshotSpreadMin (Variables|Default|GetaimShotSpreadMin))
                        (else
                          (Variables|Default|SetshotSpreadMax (Variables|Default|GethipShotSpreadMax))
                          (Variables|Default|SetshotSpreadMin (Variables|Default|GethipShotSpreadMin))))
                      (bind (_outhit _returnvalue_6) (Collision|LineTraceByChannel (Transformation|GetWorldLocation (Variables|/Game/ThirdPersonBP/Blueprints/ThirdPersonCharacter.ThirdPersonCharacter_C|GetFollowCamera (Variables|Default|Getplayer))) (Math|Vector|MakeVector (+ _x (Math|Random|RandomFloatinRange (Variables|Default|GetshotSpreadMin) (Variables|Default|GetshotSpreadMax))) (+ _y (Math|Random|RandomFloatinRange (Variables|Default|GetshotSpreadMin) (Variables|Default|GetshotSpreadMax))) (+ _z (Math|Random|RandomFloatinRange (Variables|Default|GetshotSpreadMin) (Variables|Default|GetshotSpreadMax)))) "TraceTypeQuery1" false 0 "ForDuration"))
                      (if _returnvalue_6
                        (Development|PrintString "firing")
                        (Variables|Default|SetlongBulletInClip (- (Variables|Default|GetlongBulletInClip) 1))
                        (Game|SpawnActorfromClass "/Game/Blueprints/Bullets/sniperBullet_BP.sniperBullet_BP_C" (Math|Transform|MakeTransform _returnvalue (Math|Rotator|FindLookatRotation _returnvalue (Math|Vector|SelectVector (.ImpactPoint (Collision|BreakHitResult _outhit)) (.TraceEnd (Collision|BreakHitResult _outhit)) _returnvalue_6))) "Undefined" 0 0)
                        (Audio|PlaySoundatLocation "/Game/SFX/SRFire_PH_SFX.SRFire_PH_SFX" _returnvalue)
                        (Variables|Default|SetspawnProjectile false)
                        (Utilities|FlowControl|Delay (Variables|Default|GetgunCockTime))
                        (Variables|Default|SetspawnProjectile true)))))))))))))

(event Custom|chargeShot)

(event Custom|releaseTrigger
  (bind _projectilespawnpoint (Variables|Default|GetProjectileSpawnPoint))
  (bind _player (Variables|Default|Getplayer))
  (bind _returnvalue (Transformation|GetWorldLocation _projectilespawnpoint))
  (bind _followcamera (Variables|/Game/ThirdPersonBP/Blueprints/ThirdPersonCharacter.ThirdPersonCharacter_C|GetFollowCamera _player))
  (bind _returnvalue_2 (Math|Vector|GetForwardVector _followcamera))
  (bind _returnvalue_3 (Transformation|GetWorldLocation _followcamera))
  (bind _returnvalue_4 (* _returnvalue_2 1e+04))
  (bind _returnvalue_5 (+ _returnvalue_3 _returnvalue_4))
  (bind (_x _y _z) (Math|Vector|BreakVector _returnvalue_5))
  ;[1 1 1] Firing Projectile
  (Utilities|FlowControl|Gate true) ; enters at Close
)

(event EventBeginPlay
  (bind _asthird_person_character (Utilities|Casting|CastToThirdPersonCharacter (Game|GetPlayerCharacter 0)))
  (Variables|Default|Setplayer _asthird_person_character))

(fn ConstructionScript)

(fn Reload
  (if (> (Variables|Default|GetmaxSniperAmmo) 0)
    (if (not (== (Variables|Default|GetlongBulletInClip) (Variables|Default|GetclipSize)))
      (if (> (Variables|Default|GetmaxSniperAmmo) (Variables|Default|GetclipSize))
        (bind _asthird_person_character (Utilities|Casting|CastToThirdPersonCharacter (Game|GetPlayerCharacter 0)))
        (bind _output_get (Variables|/Game/ThirdPersonBP/Blueprints/ThirdPersonCharacter.ThirdPersonCharacter_C|SetisReloading _asthird_person_character true))
        (if (and (< (Variables|Default|GetlongBulletInClip) 30) (> (Variables|Default|GetlongBulletInClip) 0)) ; Check for Conservative Ammo
          (Variables|Default|SetmaxSniperAmmo (- (Variables|Default|GetmaxSniperAmmo) (- (Variables|Default|GetclipSize) (Variables|Default|GetlongBulletInClip))))
          (Variables|Default|SetlongBulletInClip (Variables|Default|GetclipSize))
          (return _output_get false)
          (elif (<= (Variables|Default|GetlongBulletInClip) 0) ; Check if clip is empty
            (Variables|Default|SetmaxSniperAmmo (- (Variables|Default|GetmaxSniperAmmo) (Variables|Default|GetclipSize)))
            (Variables|Default|SetlongBulletInClip (Variables|Default|GetclipSize))
            (return _output_get false)))
        (else
          (Variables|Default|SetlongBulletInClip (Variables|Default|GetmaxSniperAmmo))
          (Variables|Default|SetmaxSniperAmmo 0)
          (bind _asthird_person_character_2 (Utilities|Casting|CastToThirdPersonCharacter (Game|GetPlayerCharacter 0)))
          (bind _output_get_2 (Variables|/Game/ThirdPersonBP/Blueprints/ThirdPersonCharacter.ThirdPersonCharacter_C|SetisReloading _asthird_person_character_2 true))
          (return false _output_get_2))))))