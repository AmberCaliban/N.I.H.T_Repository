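; Assault rifle weapon for the player's ThirdPersonCharacter, with automatic fire, aim-dependent spread and ammo reloading.
; Trigger events drive a Gate and RetriggerableDelay loop that fires repeatedly unless the character is reloading or the clip is empty.
; Each shot traces from the follow camera with random spread, spawning a muzzle bullet toward the impact only on a hit.
; Reload refills the clip from reserve, plays reload sounds and sets the character's IsReloading flag.
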(event Custom|pullTrigger
  (bind _skeletalmesh (Variables|Default|GetSkeletalMesh))
  (bind _character (Variables|Default|Getcharacter))
  (bind _returnvalue (Transformation|GetSocketLocation _skeletalmesh "Muzzle"))
  (bind _followcamera (Variables|/Game/ThirdPersonBP/Blueprints/ThirdPersonCharacter.ThirdPersonCharacter_C|GetFollowCamera _character))
  (bind _returnvalue_2 (Math|Vector|GetForwardVector _followcamera))
  (bind _returnvalue_3 (Transformation|GetWorldLocation _followcamera))
  (bind _returnvalue_4 (* _returnvalue_2 1e+04))
  (bind _returnvalue_5 (+ _returnvalue_3 _returnvalue_4))
  (bind (_x _y _z) (Math|Vector|BreakVector _returnvalue_5))
  ;[1 1 1] Firing Projectile
  (Utilities|FlowControl|Sequence
    (:then_0
      (goto _label Open))
    (:then_1
      (Utilities|FlowControl|Gate true :!label _label
        (:Exit
          (Utilities|FlowControl|Sequence
            (:then_0
              (Utilities|FlowControl|RetriggerableDelay 0.1)
              (goto _label))
            (:then_1
              (if (Math|Boolean|Equal(Boolean) (Variables|/Game/ThirdPersonBP/Blueprints/ThirdPersonCharacter.ThirdPersonCharacter_C|GetisReloading (Variables|Default|Getcharacter)) false)
                (if (<= (Variables|Default|GetbulletInClip) 0)
                  (Audio|PlaySoundatLocation "/Game/SFX/ARFireDry_PH_SFX.ARFireDry_PH_SFX" (Transformation|GetSocketLocation (Variables|Default|GetSkeletalMesh) "Muzzle"))
                  (Development|PrintString "Rifle Clip Empty" true false "(R=1.000000,G=0.082907,B=0.198921,A=1.000000)")
                  (else
                    (if (Variables|/Game/ThirdPersonBP/Blueprints/ThirdPersonCharacter.ThirdPersonCharacter_C|GetisAiming _character)
                      (Variables|Default|SetshotSpreadMax (Variables|Default|GetaimShotSpreadMax))
                      (Variables|Default|SetshotSpreadMin (Variables|Default|GetaimShotSpreadMin))
                      (else
                        (Variables|Default|SetshotSpreadMax (Variables|Default|GethipShotSpreadMax))
                        (Variables|Default|SetshotSpreadMin (Variables|Default|GethipShotSpreadMin))))
                    (bind (_outhit _returnvalue_6) (Collision|LineTraceByChannel _returnvalue_3 (Math|Vector|MakeVector (+ _x (Math|Random|RandomFloatinRange (Variables|Default|GetshotSpreadMin) (Variables|Default|GetshotSpreadMax))) (+ _y (Math|Random|RandomFloatinRange (Variables|Default|GetshotSpreadMin) (Variables|Default|GetshotSpreadMax))) (+ _z (Math|Random|RandomFloatinRange (Variables|Default|GetshotSpreadMin) (Variables|Default|GetshotSpreadMax)))) "TraceTypeQuery1" false 0 "ForDuration"))
                    (if _returnvalue_6
                      (Variables|Default|SetbulletInClip (- (Variables|Default|GetbulletInClip) 1))
                      (Game|SpawnActorfromClass "/Game/Blueprints/Bullets/rifleBullet_BP.rifleBullet_BP_C" (Math|Transform|MakeTransform _returnvalue (Math|Rotator|FindLookatRotation _returnvalue (Math|Vector|SelectVector (.ImpactPoint (Collision|BreakHitResult _outhit)) (.TraceEnd (Collision|BreakHitResult _outhit)) _returnvalue_6))) "Undefined" 0 0)
                      (Audio|PlaySoundatLocation "/Game/SFX/ARFire_PH_SFX.ARFire_PH_SFX" _returnvalue)
                      (Variables|Default|SetspawnProjectile false)
                      (Utilities|FlowControl|Delay 0.1)
                      (Variables|Default|SetspawnProjectile true))))
                (else
                  (Development|PrintString "cannot shoot while reloading"))))))))))

(event Custom|releaseTrigger
  (bind _skeletalmesh (Variables|Default|GetSkeletalMesh))
  (bind _character (Variables|Default|Getcharacter))
  (bind _returnvalue (Transformation|GetSocketLocation _skeletalmesh "Muzzle"))
  (bind _followcamera (Variables|/Game/ThirdPersonBP/Blueprints/ThirdPersonCharacter.ThirdPersonCharacter_C|GetFollowCamera _character))
  (bind _returnvalue_2 (Math|Vector|GetForwardVector _followcamera))
  (bind _returnvalue_3 (Transformation|GetWorldLocation _followcamera))
  (bind _returnvalue_4 (* _returnvalue_2 1e+04))
  (bind _returnvalue_5 (+ _returnvalue_3 _returnvalue_4))
  (bind (_x _y _z) (Math|Vector|BreakVector _returnvalue_5))
  ;[1 1 1] Firing Projectile
  (Utilities|FlowControl|Gate true) ; enters at Close
)

(event EventBeginPlay
  (bind _asthird_person_character (Utilities|Casting|CastToThirdPersonCharacter (Game|GetPlayerCharacter 0)))
  (Variables|Default|Setcharacter _asthird_person_character))

(fn ConstructionScript)

(fn Reload
  (if (> (Variables|Default|GetmaxAmmo) 0) ; Check if there is still ammo left in reserve
    (if (not (== (Variables|Default|GetbulletInClip) (Variables|Default|GetclipSize))) ; Check if clip is at maximum capacity
      (if (> (Variables|Default|GetmaxAmmo) (Variables|Default|GetclipSize)) ; Check if reserve ammo is more than clip size
        (bind _asthird_person_character (Utilities|Casting|CastToThirdPersonCharacter (Game|GetPlayerCharacter 0)))
        (bind _output_get (Variables|/Game/ThirdPersonBP/Blueprints/ThirdPersonCharacter.ThirdPersonCharacter_C|SetisReloading _asthird_person_character true))
        (if (and (< (Variables|Default|GetbulletInClip) 30) (> (Variables|Default|GetbulletInClip) 0)) ; Check for Conservative Reload
          (Audio|PlaySoundatLocation "/Game/SFX/ARHalfReload_PH_SFX.ARHalfReload_PH_SFX" (Transformation|GetSocketLocation (Variables|Default|GetSkeletalMesh) "Muzzle"))
          (Variables|Default|SetmaxAmmo (- (Variables|Default|GetmaxAmmo) (- (Variables|Default|GetclipSize) (Variables|Default|GetbulletInClip))))
          (Variables|Default|SetbulletInClip (Variables|Default|GetclipSize))
          (return _output_get false)
          (elif (<= (Variables|Default|GetbulletInClip) 0) ; Check for Full Reload
            (Audio|PlaySoundatLocation "/Game/SFX/ARFullReload_PH_SFX.ARFullReload_PH_SFX" (Transformation|GetSocketLocation (Variables|Default|GetSkeletalMesh) "Muzzle"))
            (Variables|Default|SetmaxAmmo (- (Variables|Default|GetmaxAmmo) (Variables|Default|GetclipSize)))
            (Variables|Default|SetbulletInClip (Variables|Default|GetclipSize))
            (return _output_get false)))
        (else
          (Audio|PlaySoundatLocation "/Game/SFX/ARFullReload_PH_SFX.ARFullReload_PH_SFX" (Transformation|GetSocketLocation (Variables|Default|GetSkeletalMesh) "Muzzle"))
          (Variables|Default|SetbulletInClip (Variables|Default|GetmaxAmmo))
          (Variables|Default|SetmaxAmmo 0)
          (bind _asthird_person_character_2 (Utilities|Casting|CastToThirdPersonCharacter (Game|GetPlayerCharacter 0)))
          (bind _output_get_2 (Variables|/Game/ThirdPersonBP/Blueprints/ThirdPersonCharacter.ThirdPersonCharacter_C|SetisReloading _asthird_person_character_2 true))
          (return false _output_get_2))))))