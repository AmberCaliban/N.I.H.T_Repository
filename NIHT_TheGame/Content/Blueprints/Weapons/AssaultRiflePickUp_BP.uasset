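; Assault rifle pickup actor that offers itself to the third-person player and holds its own reload logic.
; Overlap toggles input and the player's CanPickUpAR flag, showing the PickUp prompt only while unequipped.
; Reload flags the player as reloading, plays half or full reload audio at the muzzle, and refills the clip from reserve.
; When reserve is no larger than a clip, it replaces the clip's count instead of topping it up.
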(event Collision|EventActorBeginOverlap
  (params (OtherActor :type Actor%20Object%20Reference))
  ;[1 1 1] Pick-up set-up & Prompt
  (Utilities|Casting|CastToThirdPersonCharacter OtherActor)
  (Input|EnableInput (Game|GetPlayerController 0))
  (if (not (Variables|Default|Getequipped))
    (Rendering|SetVisibility (Variables|Default|GetPick%20up) true false)
    (Variables|/Game/ThirdPersonBP/Blueprints/ThirdPersonCharacter.ThirdPersonCharacter_C|SetcanPickUpAR (Variables|Default|Getplayer) true)))

(event EventBeginPlay
  (bind _asthird_person_character (Utilities|Casting|CastToThirdPersonCharacter (Game|GetPlayerCharacter 0)))
  (Variables|Default|Setplayer _asthird_person_character))

(event Collision|EventActorEndOverlap
  (params (OtherActor :type Actor%20Object%20Reference))
  ;[1 1 1] Pick-up set-up & Prompt
  (Utilities|Casting|CastToThirdPersonCharacter OtherActor)
  (Input|DisableInput (Game|GetPlayerController 0))
  (Rendering|SetVisibility (Variables|Default|GetPick%20up) false false)
  (Variables|/Game/ThirdPersonBP/Blueprints/ThirdPersonCharacter.ThirdPersonCharacter_C|SetcanPickUpAR (Variables|Default|Getplayer) false))

(fn ConstructionScript)

(fn Reload
  (if (> (Variables|Default|GetmaxAmmo) 0) ; Check if there is still ammo left in reserve
    (if (not (== (Variables|Default|GetbulletInClip) (Variables|Default|GetclipSize))) ; Check if clip is at maximum capacity
      (if (> (Variables|Default|GetmaxAmmo) (Variables|Default|GetclipSize)) ; Check if reserve ammo is more than clip size
        (bind _asthird_person_character (Utilities|Casting|CastToThirdPersonCharacter (Game|GetPlayerCharacter 0)))
        (bind _output_get (Variables|/Game/ThirdPersonBP/Blueprints/ThirdPersonCharacter.ThirdPersonCharacter_C|SetisReloading _asthird_person_character true))
        (if (and (< (Variables|Default|GetbulletInClip) 30) (> (Variables|Default|GetbulletInClip) 0)) ; Check for Conservative Reload
          (Audio|PlaySoundatLocation "/Game/SFX/ARHalfReload_PH_SFX.ARHalfReload_PH_SFX" (Transformation|GetSocketLocation (Variables|Default|GetSkeletalMesh) "Muzzle"))
          (Variables|Default|SetmaxAmmo (- (Variables|Default|GetmaxAmmo) (- (Variables|Default|GetclipSize) (Variables|Default|GetbulletInClip))))
          (Variables|Default|SetbulletInClip (Variables|Default|GetclipSize))
          (return _output_get false)
          (elif (<= (Variables|Default|GetbulletInClip) 0) ; Check for Full Reload
            (Audio|PlaySoundatLocation "/Game/SFX/ARFullReload_PH_SFX.ARFullReload_PH_SFX" (Transformation|GetSocketLocation (Variables|Default|GetSkeletalMesh) "Muzzle"))
            (Variables|Default|SetmaxAmmo (- (Variables|Default|GetmaxAmmo) (Variables|Default|GetclipSize)))
            (Variables|Default|SetbulletInClip (Variables|Default|GetclipSize))
            (return _output_get false)))
        (else
          (Audio|PlaySoundatLocation "/Game/SFX/ARFullReload_PH_SFX.ARFullReload_PH_SFX" (Transformation|GetSocketLocation (Variables|Default|GetSkeletalMesh) "Muzzle"))
          (Variables|Default|SetbulletInClip (Variables|Default|GetmaxAmmo))
          (Variables|Default|SetmaxAmmo 0)
          (bind _asthird_person_character_2 (Utilities|Casting|CastToThirdPersonCharacter (Game|GetPlayerCharacter 0)))
          (bind _output_get_2 (Variables|/Game/ThirdPersonBP/Blueprints/ThirdPersonCharacter.ThirdPersonCharacter_C|SetisReloading _asthird_person_character_2 true))
          (return false _output_get_2))))))