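; Sniper rifle bullet actor that deals damage on overlap, sorting what it hits by actor tag.
; Obstruction hits spawn an explosion particle effect and destroy the bullet.
; Enemy and ExplosiveBarrel hits apply the sniper rifle damage without destroying the bullet, so this graph lets it carry on through them.
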(event EventBeginPlay)

(event Collision|EventActorBeginOverlap
  (params (OtherActor :type Actor%20Object%20Reference))
  (if (Actor|ActorHasTag OtherActor "Obstruction")
    (Effects|SpawnEmitteratLocation "/Game/StarterContent/Particles/P_Explosion.P_Explosion" (Transformation|GetActorLocation))
    (Actor|DestroyActor)
    (elif (Actor|ActorHasTag OtherActor "Enemy")
      (Game|Damage|ApplyDamage OtherActor (Variables|Default|GetsniperRifleDamage) 0 0)
      (elif (Actor|ActorHasTag OtherActor "ExplosiveBarrel")
        (Game|Damage|ApplyDamage OtherActor (Variables|Default|GetsniperRifleDamage) 0 0)))))

(fn ConstructionScript)