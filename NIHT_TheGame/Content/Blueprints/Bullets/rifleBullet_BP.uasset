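; Assault rifle bullet Blueprint that applies damage and impact effects when its collision component overlaps a tagged actor.
; An overlap handler branches on actor tags: obstructions trigger an explosion emitter and destroy the bullet, while enemies, explosive barrels and DM actors take rifle damage.
; Enemy and DM hits also spawn emitters, but only DM hits pass the bullet as damage causer and destroy it, so it survives enemy and barrel overlaps.
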(event OnComponentBeginOverlap(collision)
  (params (OverlappedComponent :type Primitive%20Component%20Object%20Reference) (OtherActor :type Actor%20Object%20Reference) (OtherComp :type Primitive%20Component%20Object%20Reference) (OtherBodyIndex :type Integer) (bFromSweep :type Boolean) (SweepResult :type Hit%20Result%20Structure%20%28by%20ref%29))
  (bind _returnvalue (Transformation|GetActorLocation))
  (if (Actor|ActorHasTag OtherActor "Obstruction")
    (Effects|SpawnEmitteratLocation "/Game/StarterContent/Particles/P_Explosion.P_Explosion" _returnvalue)
    (Actor|DestroyActor)
    (elif (Actor|ActorHasTag OtherActor "Enemy")
      (Game|Damage|ApplyDamage OtherActor (Variables|Default|GetassaultRifleDamage) 0 0)
      (Effects|SpawnEmitteratLocation "/Game/VFX/Effects/Explosion.Explosion" _returnvalue)
      (elif (Actor|ActorHasTag OtherActor "ExplosiveBarrel")
        (Game|Damage|ApplyDamage OtherActor (Variables|Default|GetassaultRifleDamage) 0 0)
        (elif (Actor|ActorHasTag OtherActor "DM")
          (Game|Damage|ApplyDamage OtherActor (Variables|Default|GetassaultRifleDamage) 0 self)
          (Effects|SpawnEmitteratLocation "/Game/StarterContent/Particles/P_Explosion.P_Explosion" (Transformation|GetActorLocation))
          (Actor|DestroyActor))))))

(event EventBeginPlay)

(fn ConstructionScript)