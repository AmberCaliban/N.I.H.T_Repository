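; Dungeon room actor that shuts a door behind the player while enemies are inside and opens it once the room is clear.
; On boundary overlap it stores the ThirdPersonCharacter and, if enemies are present, locks after a short delay by showing the door with collision enabled.
; Tick box-tests the boundary for pawns, ignoring the stored player, to update EnemiesPresent.
; The first empty result triggers a delayed unlock through a DoOnce that is never reset.
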(event OnComponentBeginOverlap(roomBoundary)
  (params (OverlappedComponent :type Primitive%20Component%20Object%20Reference) (OtherActor :type Actor%20Object%20Reference) (OtherComp :type Primitive%20Component%20Object%20Reference) (OtherBodyIndex :type Integer) (bFromSweep :type Boolean) (SweepResult :type Hit%20Result%20Structure%20%28by%20ref%29))
  (bind _asthird_person_character (Utilities|Casting|CastToThirdPersonCharacter OtherActor))
  (Variables|Default|Setplayer _asthird_person_character)
  (if (Variables|Default|GetenemiesPresent)
    (Utilities|FlowControl|Delay 1.0)
    (CallFunction|LockRoom)
    (Development|PrintString "locked")
    (else
      (Development|PrintString "no more"))))

(event Custom|lockRoom
  (bind _door (Variables|Default|GetDoor))
  ;[1 1 1] Lock Dungeon
  (Rendering|SetVisibility _door true false)
  (Collision|SetCollisionEnabled _door "QueryAndPhysics"))

(event Custom|unlockRoom
  (bind _door (Variables|Default|GetDoor))
  ;[1 1 1] Unlock Dungeon
  (Utilities|FlowControl|Delay 2.0)
  (Rendering|SetVisibility _door false false)
  (Collision|SetCollisionEnabled _door "NoCollision"))

(event EventTick
  (params (DeltaSeconds :type Float%20%28single-precision%29))
  (bind _roomboundary (Variables|Default|GetroomBoundary))
  (bind _returnvalue (Collision|BoxOverlapActors (Transformation|GetWorldLocation _roomboundary) (Components|Box|GetScaledBoxExtent _roomboundary) (Utilities|Array|MakeArray "ObjectTypeQuery3") 0 (Utilities|Array|MakeArray (Variables|Default|Getplayer)) :!class /Script/Engine.KismetSystemLibrary))
  (if _returnvalue
    (Variables|Default|SetenemiesPresent true)
    (else
      (Variables|Default|SetenemiesPresent false)
      (Utilities|FlowControl|DoOnce false
        (:Completed
          (CallFunction|UnlockRoom))))))

(fn ConstructionScript)