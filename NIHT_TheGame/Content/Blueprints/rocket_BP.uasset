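; Homing rocket projectile that chases the player character and explodes with radial damage.
; After a short launch delay, it turns on ProjectileMovement homing toward the player's mesh and snaps its rotation to face them once.
; It detonates on capsule overlap with a Player or Obstruction tag, or when its lifespan runs out after homing starts.
; Explosion spawns effects, applies falloff damage and destroys the actor; its debug-drawn sphere trace result is unused.
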(event OnComponentBeginOverlap(Capsule)
  (params (OverlappedComponent :type Primitive%20Component%20Object%20Reference) (OtherActor :type Actor%20Object%20Reference) (OtherComp :type Primitive%20Component%20Object%20Reference) (OtherBodyIndex :type Integer) (bFromSweep :type Boolean) (SweepResult :type Hit%20Result%20Structure%20%28by%20ref%29))
  (if (Actor|ActorHasTag OtherActor "Player")
    (CallFunction|Explosion :!label _label)
    (elif (Actor|ActorHasTag OtherActor "Obstruction")
      (goto _label))))

(event Custom|Explosion
  (bind _returnvalue (Transformation|GetActorLocation))
  (bind _rocketmesh (Variables|Default|GetrocketMesh))
  (bind _returnvalue_2 (Transformation|GetWorldLocation _rocketmesh))
  (Collision|MultiSphereTraceForObjects _returnvalue_2 _returnvalue_2 2e+02 (Utilities|Array|MakeArray "ObjectTypeQuery3") false 0 "ForDuration")
  (Effects|SpawnEmitteratLocation "/Game/StarterContent/Particles/P_Explosion.P_Explosion" _returnvalue)
  (Audio|PlaySoundatLocation "/Game/StarterContent/Audio/Explosion01.Explosion01" _returnvalue)
  (Class|GameplayStatics|ApplyRadialDamagewithFalloff 15.0 1e+01 _returnvalue 5e+01 2e+02 0.5 0 0 0 0 "ECC_Visibility")
  (Actor|DestroyActor))

(event EventBeginPlay
  (bind _projectilemovement (Variables|Default|GetProjectileMovement))
  ;[1 1 1] Home onto Player
  (bind _asthird_person_character (Utilities|Casting|CastToThirdPersonCharacter (Game|GetPlayerCharacter 0)))
  (Variables|Default|Setcharacter _asthird_person_character)
  (Utilities|FlowControl|Delay 0.8)
  (Variables|/Script/Engine.ProjectileMovementComponent|SetHomingTargetComponent _projectilemovement (Variables|/Script/Engine.Character|GetMesh (Variables|Default|Getcharacter)))
  (Variables|/Script/Engine.ProjectileMovementComponent|SetHomingAccelerationMagnitude _projectilemovement 5e+03)
  (Variables|/Script/Engine.ProjectileMovementComponent|SetbIsHomingProjectile _projectilemovement true)
  (Transformation|SetActorRotation (Math|Rotator|FindLookatRotation (Transformation|GetActorLocation) (Transformation|GetActorLocation (Variables|Default|Getcharacter))))
  (Utilities|FlowControl|Delay (Variables|Default|GetrocketLifeSpan))
  (CallFunction|Explosion))

(fn ConstructionScript)