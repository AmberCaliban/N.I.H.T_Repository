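; Rocket projectile actor that can home in on the player's third-person character and explodes on overlap with actors tagged Player or Obstruction.
; BeginPlay caches the character, and the HomingMissile event plays a timeline that lerps the rocket toward that character's current location, printing the location each update.
; A delay triggered from those updates destroys the rocket after half a second, without the explosion effect and sound used on overlap.
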(event Custom|Homing%20Missile
  (bind _character (Variables|Default|Getcharacter))
  (bind _returnvalue (Transformation|GetActorLocation _character))
  (bind _newtrack_0 (Timeline|Timeline_0 Play)
    (:Update
      (Transformation|SetActorLocation (Math|Vector|Lerp(Vector) (Transformation|GetActorLocation) _returnvalue _newtrack_0) false false)
      (Development|PrintString (Utilities|String|ToString(Vector) _returnvalue))
      (Utilities|FlowControl|Delay 0.5)
      (Actor|DestroyActor))))

(event EventBeginPlay
  (bind _asthird_person_character (Utilities|Casting|CastToThirdPersonCharacter (Game|GetPlayerCharacter 0)))
  (Variables|Default|Setcharacter _asthird_person_character))

(event Collision|EventActorBeginOverlap
  (params (OtherActor :type Actor%20Object%20Reference))
  (bind _returnvalue (Transformation|GetActorLocation))
  (if (or (Actor|ActorHasTag OtherActor "Player") (Actor|ActorHasTag OtherActor "Obstruction"))
    (Effects|SpawnEmitteratLocation "/Game/StarterContent/Particles/P_Explosion.P_Explosion" _returnvalue "0, 0, 0" "0.200000,0.200000,0.200000")
    (Audio|PlaySoundatLocation "/Game/StarterContent/Audio/Explosion01.Explosion01" _returnvalue)
    (Actor|DestroyActor)))

(event EventTick
  (params (DeltaSeconds :type Float%20%28single-precision%29)))

(fn ConstructionScript)