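; Explosive barrel prop that loses health from any damage, activates a fire component when low, and explodes at zero health.
; The explosion spawns particles and sound, applies radial damage with falloff, calls Detonate, then destroys the actor.
; Detonate sphere-traces around the barrel and launches ThirdPersonCharacter hits away and upward, with less outward and more upward force for those off the ground.
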(event EventBeginPlay)

(event EventTick
  (params (DeltaSeconds :type Float%20%28single-precision%29)))

(event Game|Damage|EventAnyDamage
  (params (Damage :type Float%20%28single-precision%29) (DamageType :type Damage%20Type%20Object%20Reference) (InstigatedBy :type Controller%20Object%20Reference) (DamageCauser :type Actor%20Object%20Reference))
  (bind _returnvalue (Transformation|GetActorLocation))
  (Development|PrintString "hit barrel")
  (bind _output_get (Variables|Default|SetbarrelHealth (- (Variables|Default|GetbarrelHealth) Damage)))
  (if (<= _output_get 0.0)
    (Effects|SpawnEmitteratLocation "/Game/StarterContent/Particles/P_Explosion.P_Explosion" _returnvalue "0, 0, 0" "3.000000,3.000000,3.000000")
    (Audio|PlaySoundatLocation "/Game/StarterContent/Audio/Explosion02.Explosion02" _returnvalue)
    (Class|GameplayStatics|ApplyRadialDamagewithFalloff (Variables|Default|GetexplosionDamage) 75.0 _returnvalue 5e+01 (Variables|Default|GetexplosionDamageRadius) 0.5 0 0 self 0 "ECC_Visibility")
    (CallFunction|Detonate)
    (Actor|DestroyActor)
    (elif (< (Variables|Default|GetbarrelHealth) 5e+01)
      (Components|Activation|Activate (Variables|Default|GetFire) false))))

(fn ConstructionScript)

(fn Detonate
  (bind _barrel (Variables|Default|GetBarrel))
  (bind _returnvalue (Transformation|GetWorldLocation _barrel))
  (bind (_outhits _returnvalue_2) (Collision|MultiSphereTraceForObjects _returnvalue _returnvalue 275.0 (Utilities|Array|MakeArray "ObjectTypeQuery3" "ObjectTypeQuery4" "ObjectTypeQuery2") false 0 "Persistent"))
  (if _returnvalue_2
    (for _array_element _outhits
      (bind _asthird_person_character (Utilities|Casting|CastToThirdPersonCharacter (.HitActor (Collision|BreakHitResult _array_element))))
      (if (AI|Components|NavMovement|IsMovingonGround (Variables|/Script/Engine.Character|GetCharacterMovement _asthird_person_character))
        (Character|LaunchCharacter _asthird_person_character (Math|Vector|MakeVector (.x (* (Math|Vector|Normalize (- (Transformation|GetActorLocation _asthird_person_character) (Transformation|GetActorLocation))) 1e+03)) (.y (* (Math|Vector|Normalize (- (Transformation|GetActorLocation _asthird_person_character) (Transformation|GetActorLocation))) 1e+03)) 1e+03) false false)
        (else
          (Character|LaunchCharacter _asthird_person_character (Math|Vector|MakeVector (.x (* (Math|Vector|Normalize (- (Transformation|GetActorLocation _asthird_person_character) (Transformation|GetActorLocation))) 5e+02)) (.y (* (Math|Vector|Normalize (- (Transformation|GetActorLocation _asthird_person_character) (Transformation|GetActorLocation))) 5e+02)) 1.5e+03) false false))))))