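; Interactive spotlight actor that the player switches on and off with the E key while inside its trigger volume.
; Trigger begin and end overlaps enable and disable the actor's input for player controller 0 and toggle the help text, without checking which actor overlaps.
; The construction script applies the spotlight's color and initial visibility from the LightColor and VisibilitySettings variables.
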(event OnComponentBeginOverlap(Trigger)
  (params (OverlappedComponent :type Primitive%20Component%20Object%20Reference) (OtherActor :type Actor%20Object%20Reference) (OtherComp :type Primitive%20Component%20Object%20Reference) (OtherBodyIndex :type Integer) (bFromSweep :type Boolean) (SweepResult :type Hit%20Result%20Structure%20%28by%20ref%29))
  ;[1 0.5378 0.4794] Enable/Disable Input & Toggle Help Text Visibility
  (Input|EnableInput (Game|GetPlayerController 0))
  (Rendering|ToggleVisibility (Variables|Default|GetHelp%20Text) false))

(event OnComponentEndOverlap(Trigger)
  (params (OverlappedComponent :type Primitive%20Component%20Object%20Reference) (OtherActor :type Actor%20Object%20Reference) (OtherComp :type Primitive%20Component%20Object%20Reference) (OtherBodyIndex :type Integer))
  ;[1 0.5378 0.4794] Enable/Disable Input & Toggle Help Text Visibility
  (Input|DisableInput (Game|GetPlayerController 0))
  (Rendering|ToggleVisibility (Variables|Default|GetHelp%20Text) false))

(event EventBeginPlay)

(event Collision|EventActorBeginOverlap
  (params (OtherActor :type Actor%20Object%20Reference)))

(event EventTick
  (params (DeltaSeconds :type Float%20%28single-precision%29)))

(event Input|KeyboardEvents|E
  (params (Key :type Key%20Structure))
  ;[0.6493 1 0.5993] Toggle Light Visibility
  (:Pressed
    (Rendering|ToggleVisibility (Variables|Default|GetSpotLight) false)))

(fn ConstructionScript
  (bind _spotlight (Variables|Default|GetSpotLight))
  (Rendering|Components|Light|SetLightColor _spotlight (Variables|Default|GetLightColor) true)
  (Rendering|SetVisibility _spotlight (Variables|Default|GetVisibility%20Settings) false))