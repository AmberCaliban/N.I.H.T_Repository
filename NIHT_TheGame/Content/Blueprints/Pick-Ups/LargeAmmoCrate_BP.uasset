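; Large ammo crate pickup that, once activated, bursts out a random mix of ammo and restoration spray pickups.
; Trigger box overlaps flag crate presence on the ThirdPersonCharacter and toggle the crate's own can-activate flag.
; AmmoCrateActivation calls SpawnAmmo only on first use, then prints that the crate is empty.
; SpawnAmmo loops, spawning a random pickup class at AmmoSpawnPoint and launching each with an upward impulse.
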(event OnComponentBeginOverlap(triggerBox)
  (params (OverlappedComponent :type Primitive%20Component%20Object%20Reference) (OtherActor :type Actor%20Object%20Reference) (OtherComp :type Primitive%20Component%20Object%20Reference) (OtherBodyIndex :type Integer) (bFromSweep :type Boolean) (SweepResult :type Hit%20Result%20Structure%20%28by%20ref%29))
  (bind _asthird_person_character (Utilities|Casting|CastToThirdPersonCharacter OtherActor))
  (Variables|/Game/ThirdPersonBP/Blueprints/ThirdPersonCharacter.ThirdPersonCharacter_C|SetammoCratePresent _asthird_person_character true)
  (Variables|Default|SetcanActivateAmmoCrate true))

(event OnComponentEndOverlap(triggerBox)
  (params (OverlappedComponent :type Primitive%20Component%20Object%20Reference) (OtherActor :type Actor%20Object%20Reference) (OtherComp :type Primitive%20Component%20Object%20Reference) (OtherBodyIndex :type Integer))
  (bind _asthird_person_character (Utilities|Casting|CastToThirdPersonCharacter OtherActor))
  (Variables|/Game/ThirdPersonBP/Blueprints/ThirdPersonCharacter.ThirdPersonCharacter_C|SetammoCratePresent _asthird_person_character false)
  (Variables|Default|SetcanActivateAmmoCrate false))

(event Custom|Spawn%20Ammo
  (bind _ammo_spawn_point (Variables|Default|GetAmmo%20Spawn%20Point))
  (bind _returnvalue (Transformation|GetWorldTransform _ammo_spawn_point))
  (for _index (range 0 3)
    (switch int (Math|Random|RandomIntegerinRange 0 3) ; Randomise Spawning of ammo
      (:0
        (bind _returnvalue_2 (Game|SpawnActorfromClass "/Game/Blueprints/Pick-Ups/Ammo/ARAmmo_BP.ARAmmo_BP_C" _returnvalue "Undefined" 0 0))
        ;[1 1 1] Make Ammo fly into air
        (Physics|AddImpulse (Variables|/Game/Blueprints/Pick-Ups/Ammo/ARAmmo_BP.ARAmmo_BP_C|GetrifleAmmo _returnvalue_2) "0, 0,500.000000" "None" false))
      (:1
        (bind _returnvalue_3 (Game|SpawnActorfromClass "/Game/Blueprints/Pick-Ups/Ammo/SGAmmo_BP.SGAmmo_BP_C" _returnvalue "Undefined" 0 0))
        (Physics|AddImpulse (Variables|/Game/Blueprints/Pick-Ups/Ammo/SGAmmo_BP.SGAmmo_BP_C|GetshotgunAmmo _returnvalue_3) "0, 0,500.000000" "None" false))
      (:2
        (bind _returnvalue_4 (Game|SpawnActorfromClass "/Game/Blueprints/Pick-Ups/Ammo/SRAmmo_BP.SRAmmo_BP_C" _returnvalue "Undefined" 0 0))
        (Physics|AddImpulse (Variables|/Game/Blueprints/Pick-Ups/Ammo/SRAmmo_BP.SRAmmo_BP_C|GetrifleAmmo _returnvalue_4) "0, 0,500.000000" "None" false))
      (:3
        (bind _returnvalue_5 (Game|SpawnActorfromClass "/Game/Blueprints/Pick-Ups/RestorationSpray_BP.RestorationSpray_BP_C" _returnvalue "Undefined" 0 0))
        (Physics|AddImpulse (Variables|/Game/Blueprints/Pick-Ups/RestorationSpray_BP.RestorationSpray_BP_C|GetRestorationSpray_PH _returnvalue_5) "0, 0,500.000000" "None" false)))))

(event EventBeginPlay)

(event Collision|EventActorBeginOverlap
  (params (OtherActor :type Actor%20Object%20Reference)))

(event EventTick
  (params (DeltaSeconds :type Float%20%28single-precision%29)))

(event EventAmmoCrateActivation
  ;[1 1 1] Calling Spawn Ammo
  (if (Variables|Default|GetcrateOpened)
    (Development|PrintString "Crate Empty!" true true "(R=1.000000,G=0.066983,B=0.125737,A=1.000000)")
    (else
      (CallFunction|SpawnAmmo)
      (Variables|Default|SetcrateOpened true))))

(fn ConstructionScript)