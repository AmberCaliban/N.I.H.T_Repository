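; Assault rifle ammo pick-up that replenishes the player's reserve rifle ammo.
; BeginPlay caches the player character, and a Hitbox overlap by a ThirdPersonCharacter calls AddAmmo only while that player has the rifle equipped.
; AddAmmo adds a set amount to the weapon's MaxAmmo, capped at MaxAmmoStorage, then destroys the pick-up.
; When storage is already full, the pick-up stays in the world.
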(event OnComponentBeginOverlap(Hitbox)
  (params (OverlappedComponent :type Primitive%20Component%20Object%20Reference) (OtherActor :type Actor%20Object%20Reference) (OtherComp :type Primitive%20Component%20Object%20Reference) (OtherBodyIndex :type Integer) (bFromSweep :type Boolean) (SweepResult :type Hit%20Result%20Structure%20%28by%20ref%29))
  ;[1 1 1] Check Collision with Player
  (Utilities|Casting|CastToThirdPersonCharacter OtherActor)
  (if (Utilities|IsValid (Variables|Default|Getplayer))
    (if (Variables|/Game/ThirdPersonBP/Blueprints/ThirdPersonCharacter.ThirdPersonCharacter_C|GetrifleEquipped (Variables|Default|Getplayer))
      (CallFunction|AddAmmo))))

(event Custom|Add%20Ammo
  (bind _player (Variables|Default|Getplayer))
  (bind _weapon (Variables|/Game/ThirdPersonBP/Blueprints/ThirdPersonCharacter.ThirdPersonCharacter_C|GetWeapon _player))
  ;[1 1 1] Assault Rifle Ammo Replenishment
  (if (< (Variables|/Game/Blueprints/Weapons/AssaultRifle_BP.AssaultRifle_BP_C|GetmaxAmmo (Variables|/Game/ThirdPersonBP/Blueprints/ThirdPersonCharacter.ThirdPersonCharacter_C|GetWeapon (Variables|Default|Getplayer))) (Variables|Default|GetmaxAmmoStorage)) ; Check if total rifle ammo on player is less than maximum
    (if (>= (- (Variables|Default|GetmaxAmmoStorage) (Variables|/Game/Blueprints/Weapons/AssaultRifle_BP.AssaultRifle_BP_C|GetmaxAmmo (Variables|/Game/ThirdPersonBP/Blueprints/ThirdPersonCharacter.ThirdPersonCharacter_C|GetWeapon (Variables|Default|Getplayer)))) (Variables|Default|GetammoToReplenish)) ; Check if amount of depleted ammo is more than amount pick up will replenish
      (Variables|/Game/Blueprints/Weapons/AssaultRifle_BP.AssaultRifle_BP_C|SetmaxAmmo _weapon (+ (Variables|/Game/Blueprints/Weapons/AssaultRifle_BP.AssaultRifle_BP_C|GetmaxAmmo _weapon) (Variables|Default|GetammoToReplenish))) ; Add onto current Max Ammo
      (Actor|DestroyActor :!label _label) ; Destroy Ammo if it is collected
      (elif (< (- (Variables|Default|GetmaxAmmoStorage) (Variables|/Game/Blueprints/Weapons/AssaultRifle_BP.AssaultRifle_BP_C|GetmaxAmmo (Variables|/Game/ThirdPersonBP/Blueprints/ThirdPersonCharacter.ThirdPersonCharacter_C|GetWeapon (Variables|Default|Getplayer)))) (Variables|Default|GetammoToReplenish)) ; Check if less than all replenished ammo is needed to replenish to full ammo
        (Variables|/Game/Blueprints/Weapons/AssaultRifle_BP.AssaultRifle_BP_C|SetmaxAmmo (Variables|/Game/ThirdPersonBP/Blueprints/ThirdPersonCharacter.ThirdPersonCharacter_C|GetWeapon (Variables|Default|Getplayer)) (Variables|Default|GetmaxAmmoStorage)) ; Set Max Ammo to Max Storage Amount
        (goto _label)))))

(event EventBeginPlay
  (bind _asthird_person_character (Utilities|Casting|CastToThirdPersonCharacter (Game|GetPlayerCharacter 0)))
  (Variables|Default|Setplayer _asthird_person_character)
  (Variables|Default|Setrifle (Variables|/Game/ThirdPersonBP/Blueprints/ThirdPersonCharacter.ThirdPersonCharacter_C|GetWeapon _asthird_person_character)))

(fn ConstructionScript)