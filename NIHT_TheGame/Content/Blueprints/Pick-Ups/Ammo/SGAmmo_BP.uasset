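; Shotgun shell pickup that replenishes the player's reserve shells when the player walks into it.
; Hitbox overlap casts the actor to ThirdPersonCharacter, then AddAmmo runs only if that player's shotgun is valid, equipped and below the storage maximum.
; It adds the replenish amount, capped at the maximum, and destroys itself only when shells are actually granted.
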(event OnComponentBeginOverlap(Hitbox)
  (params (OverlappedComponent :type Primitive%20Component%20Object%20Reference) (OtherActor :type Actor%20Object%20Reference) (OtherComp :type Primitive%20Component%20Object%20Reference) (OtherBodyIndex :type Integer) (bFromSweep :type Boolean) (SweepResult :type Hit%20Result%20Structure%20%28by%20ref%29))
  ;[1 1 1] Check Collision with Player
  (bind _asthird_person_character (Utilities|Casting|CastToThirdPersonCharacter OtherActor))
  (Variables|Default|Setplayer _asthird_person_character)
  (if true
    (CallFunction|AddAmmo)))

(event Custom|Add%20Ammo
  (bind _player (Variables|Default|Getplayer))
  (bind _player_2 (Variables|Default|Getplayer))
  (bind _shotgun (Variables|/Game/ThirdPersonBP/Blueprints/ThirdPersonCharacter.ThirdPersonCharacter_C|GetShotgun _player))
  (bind _shotgun_2 (Variables|/Game/ThirdPersonBP/Blueprints/ThirdPersonCharacter.ThirdPersonCharacter_C|GetShotgun _player_2))
  ;[1 1 1] Shotgun Shell Replenishment
  (if (Utilities|IsValid _shotgun_2)
    (if (and (Variables|/Game/ThirdPersonBP/Blueprints/ThirdPersonCharacter.ThirdPersonCharacter_C|GetshotgunEquipped _player_2) (< (Variables|/Game/Blueprints/Weapons/Shotgun_BP.Shotgun_BP_C|GetmaxShotgunShell _shotgun_2) (Variables|Default|GetmaxShellStorage))) ; Check if total rifle ammo on player is less than maximum
      (if (>= (- (Variables|Default|GetmaxShellStorage) (Variables|/Game/Blueprints/Weapons/Shotgun_BP.Shotgun_BP_C|GetmaxShotgunShell (Variables|/Game/ThirdPersonBP/Blueprints/ThirdPersonCharacter.ThirdPersonCharacter_C|GetShotgun (Variables|Default|Getplayer)))) (Variables|Default|GetammoToReplenish)) ; Check if amount of depleted ammo is more than amount pick up will replenish
        (Variables|/Game/Blueprints/Weapons/Shotgun_BP.Shotgun_BP_C|SetmaxShotgunShell _shotgun (+ (Variables|/Game/Blueprints/Weapons/Shotgun_BP.Shotgun_BP_C|GetmaxShotgunShell _shotgun) (Variables|Default|GetammoToReplenish))) ; Add onto current Max Shells
        (Actor|DestroyActor :!label _label) ; Destroy Ammo if it is collected
        (elif (< (- (Variables|Default|GetmaxShellStorage) (Variables|/Game/Blueprints/Weapons/Shotgun_BP.Shotgun_BP_C|GetmaxShotgunShell (Variables|/Game/ThirdPersonBP/Blueprints/ThirdPersonCharacter.ThirdPersonCharacter_C|GetShotgun (Variables|Default|Getplayer)))) (Variables|Default|GetammoToReplenish)) ; Check if less than all replenished ammo is needed to replenish to full ammo
          (Variables|/Game/Blueprints/Weapons/Shotgun_BP.Shotgun_BP_C|SetmaxShotgunShell (Variables|/Game/ThirdPersonBP/Blueprints/ThirdPersonCharacter.ThirdPersonCharacter_C|GetShotgun (Variables|Default|Getplayer)) (Variables|Default|GetmaxShellStorage)) ; Set Max Shells to Max Shell Amount
          (goto _label))))))

(fn ConstructionScript)