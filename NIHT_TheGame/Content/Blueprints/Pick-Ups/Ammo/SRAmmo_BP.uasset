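; Sniper rifle ammo pick-up that replenishes the player's reserve sniper ammo.
; When its hitbox overlaps a ThirdPersonCharacter with the sniper equipped, it compares the sniper's MaxSniperAmmo against MaxAmmoStorage.
; If the reserve is below the cap, it adds AmmoToReplenish, clamped to that cap, then destroys itself.
; At full reserve, or without the sniper equipped, the pick-up stays in the world.
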(event OnComponentBeginOverlap(Hitbox)
  (params (OverlappedComponent :type Primitive%20Component%20Object%20Reference) (OtherActor :type Actor%20Object%20Reference) (OtherComp :type Primitive%20Component%20Object%20Reference) (OtherBodyIndex :type Integer) (bFromSweep :type Boolean) (SweepResult :type Hit%20Result%20Structure%20%28by%20ref%29))
  ;[1 1 1] Check Collision with Player
  (bind _asthird_person_character (Utilities|Casting|CastToThirdPersonCharacter OtherActor))
  (bind _output_get (Variables|Default|Setplayer _asthird_person_character))
  (if (Variables|/Game/ThirdPersonBP/Blueprints/ThirdPersonCharacter.ThirdPersonCharacter_C|GetsniperEquipped _output_get)
    (CallFunction|AddAmmo)))

(event Custom|Add%20Ammo
  (bind _player (Variables|Default|Getplayer))
  (bind _sniper (Variables|/Game/ThirdPersonBP/Blueprints/ThirdPersonCharacter.ThirdPersonCharacter_C|GetSniper _player))
  ;[1 1 1] Sniper Ammo Replenishment
  (if (< (Variables|/Game/Blueprints/Weapons/Sniper_BP.Sniper_BP_C|GetmaxSniperAmmo (Variables|/Game/ThirdPersonBP/Blueprints/ThirdPersonCharacter.ThirdPersonCharacter_C|GetSniper (Variables|Default|Getplayer))) (Variables|Default|GetmaxAmmoStorage)) ; Check if total rifle ammo on player is less than maximum storage amt
    (if (>= (- (Variables|Default|GetmaxAmmoStorage) (Variables|/Game/Blueprints/Weapons/Sniper_BP.Sniper_BP_C|GetmaxSniperAmmo (Variables|/Game/ThirdPersonBP/Blueprints/ThirdPersonCharacter.ThirdPersonCharacter_C|GetSniper (Variables|Default|Getplayer)))) (Variables|Default|GetammoToReplenish)) ; Check if amount of depleted ammo is more than amount pick up will replenish
      (Variables|/Game/Blueprints/Weapons/Sniper_BP.Sniper_BP_C|SetmaxSniperAmmo _sniper (+ (Variables|/Game/Blueprints/Weapons/Sniper_BP.Sniper_BP_C|GetmaxSniperAmmo _sniper) (Variables|Default|GetammoToReplenish))) ; Add onto current Max Ammo
      (Actor|DestroyActor :!label _label) ; Destroy Ammo if it is collected
      (elif (< (- (Variables|Default|GetmaxAmmoStorage) (Variables|/Game/Blueprints/Weapons/Sniper_BP.Sniper_BP_C|GetmaxSniperAmmo (Variables|/Game/ThirdPersonBP/Blueprints/ThirdPersonCharacter.ThirdPersonCharacter_C|GetSniper (Variables|Default|Getplayer)))) (Variables|Default|GetammoToReplenish)) ; Check if less than all replenished ammo is needed to replenish to full ammo
        (Variables|/Game/Blueprints/Weapons/Sniper_BP.Sniper_BP_C|SetmaxSniperAmmo (Variables|/Game/ThirdPersonBP/Blueprints/ThirdPersonCharacter.ThirdPersonCharacter_C|GetSniper (Variables|Default|Getplayer)) (Variables|Default|GetmaxAmmoStorage)) ; Set Max Ammo to Max Storage Amount
        (goto _label)))))

(fn ConstructionScript)